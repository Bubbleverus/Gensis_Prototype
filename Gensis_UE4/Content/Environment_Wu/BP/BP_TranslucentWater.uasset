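; BP_TranslucentWater is a translucent water surface whose size and look are driven by Blueprint variables.
; Its construction script calls InitialWaterCreation, which creates a dynamic material instance on the WaterSurface component and scales it in X and Y.
; It then pushes shore, wave, variation, depth and color settings into the material, along with the surface's world Z as water height.
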(fn `UserConstructionScript`
  (bind _watersurface (`self.WaterSurface`))
  (bind _watersurface_2 (`self.WaterSurface`))
  (bind _returnvalue (`PrimitiveComponent.CreateDynamicMaterialInstance` _watersurface 0 (`self.TranslucentWaterMaterial`)))
  (set `self.Water Material` _returnvalue)
  (`SceneComponent.SetRelativeScale3D` _watersurface (`KismetMathLibrary.MakeVector` (`self.Water Scale X`) (`self.Water Scale Y`) 1.0))
  (`MeshComponent.SetScalarParameterValueOnMaterials` _watersurface_2 "Shore Depth" (`self.Shore Depth`))
  (`MeshComponent.SetScalarParameterValueOnMaterials` _watersurface_2 "Wave Speed" (`self.Wave Speed`))
  (`MeshComponent.SetScalarParameterValueOnMaterials` _watersurface_2 "Max Shore Opacity" (`self.MaxShoreOpacity`))
  (`MeshComponent.SetScalarParameterValueOnMaterials` _watersurface_2 "Water Height" (.z (`SceneComponent.K2_GetComponentLocation` (`self.WaterSurface`))))
  (`MeshComponent.SetScalarParameterValueOnMaterials` _watersurface_2 "Variation Amount" (`self.Variation Amount`))
  (`MeshComponent.SetVectorParameterValueOnMaterials` (`self.WaterSurface`) "WaterColor A" (`KismetMathLibrary.Conv_LinearColorToVector` (`self.Primary Water Color`)))
  (`MeshComponent.SetVectorParameterValueOnMaterials` (`self.WaterSurface`) "WaterColor B" (`KismetMathLibrary.Conv_LinearColorToVector` (`self.Secondary Water Color`)))
  (`MeshComponent.SetScalarParameterValueOnMaterials` _watersurface_2 "Water Depth" (`self.Depth Scale`))
  (`MeshComponent.SetVectorParameterValueOnMaterials` (`self.WaterSurface`) "DeepWater" (`KismetMathLibrary.Conv_LinearColorToVector` (`self.Deep Water Color`)))
  (`MeshComponent.SetVectorParameterValueOnMaterials` (`self.WaterSurface`) "ShallowWater" (`KismetMathLibrary.Conv_LinearColorToVector` (`self.Shallow Water Color`))))