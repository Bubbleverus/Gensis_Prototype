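; Boss enemy Blueprint that tracks health and handles death, leaving a portal effect behind.
; AnyDamage subtracts damage from clamped health unless Blocked is set, printing the result to screen.
; At zero health it stops the AI controller's brain logic, then a DoOnce plays the death animation and disables capsule collision.
; After a delay it destroys the actor and spawns the portal particle emitter at its location.
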(event `self.ReceiveAnyDamage`
  (params (Damage :type "Float (single-precision)") (DamageType :type "DamageType Object Reference") (InstigatedBy :type "Controller Object Reference") (DamageCauser :type "Actor Object Reference"))
  (set `self.Damage` Damage)
  (if (not (`self.Blocked`))
    (bind _output_get (set `self.BossHealth` (`KismetMathLibrary.FClamp` (- (`self.BossHealth`) (`self.Damage`)) 0.0 500.0)))
    (`KismetSystemLibrary.PrintString` (`KismetStringLibrary.Conv_DoubleToString` _output_get))
    (if (<= (`self.BossHealth`) 0.0)
      (bind _returnvalue (`AIBlueprintHelperLibrary.GetAIController` self))
      (`BrainComponent.StopLogic` (`AIController.BrainComponent` _returnvalue) "Dead")
      (`/Engine/EditorBlueprintResources/StandardMacros.DoOnce` false
        (:`Completed`
          (`SkeletalMeshComponent.PlayAnimation` (`self.Mesh`) "/Game/BigBoss/BOSS_Final/Standing_React_Death_Forward.Standing_React_Death_Forward" false)
          (`PrimitiveComponent.SetCollisionEnabled` (`self.CapsuleComponent`) "NoCollision")
          (`KismetSystemLibrary.Delay` 7.0)
          (`self.K2_DestroyActor`)
          (`GameplayStatics.SpawnEmitterAtLocation` "/Game/Environment_Wu/Effects/Portal/P_Portal.P_Portal" (`self.K2_GetActorLocation`) (struct) false))))))

(fn `UserConstructionScript`)