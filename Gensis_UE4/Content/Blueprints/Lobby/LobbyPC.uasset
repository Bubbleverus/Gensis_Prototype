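; Lobby player controller that runs the lobby menu, character choice and chat for a player.
; Construction loads PlayerInfo from the save slot; BeginPlay shows the cursor and creates the lobby widget, which receives player cards.
; Character changes update PlayerInfo, save PlayerSave and ask LobbyGM to swap the character.
; Incoming chat updates this controller's own chat widget once per connected player in LobbyGM's list.
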(event `self.ReceiveBeginPlay`
  (bind _returnvalue (`GameplayStatics.GetPlayerController` 0))
  ;[1 1 1] Create a Lobby Widget OnBeginPlay
  (set `PlayerController.bShowMouseCursor` true _returnvalue)
  (bind _returnvalue_2 (`|CreateWidget` "/Game/UI/Lobby/LobbyWB.LobbyWB_C" _returnvalue))
  (bind _output_get (set `self.LobbyMenuWB` _returnvalue_2))
  (`UserWidget.AddToViewport` _output_get 0))

(event `AddPlayerInfo`
  (params (AllPlayerInfo :type "Array of /Game/Blueprints/AllLevels/PlayerInfo Structure"))
  ;[1 1 1] Add the players info to the lobby Menu
  (for _array_element AllPlayerInfo
    (`/Game/UI/Lobby/LobbyWB.AddNewPlayerCard` (`self.LobbyMenuWB`) _array_element)))

(event `AssignNewCharacter`
  (params (NewCharacter :type "Character Class Reference"))
  ;[1 1 1] Swap Character
  (setmembers `/Game/Blueprints/AllLevels/PlayerInfo` :`StructRef` (`self.PlayerInfo`) :`LastUsedCharacter` NewCharacter)
  (`GameplayStatics.SaveGameToSlot` (`self.PlayerSave`) "PlayerSaveGame")
  (`/Game/Blueprints/Lobby/LobbyGM.SwapCharacter` (cast `/Game/Blueprints/Lobby/LobbyGM` (`GameplayStatics.GetGameMode`) :!pure true) NewCharacter self))

(event `GetChatMessage`
  (params (MessageToSend :type Text))
  ;[1 1 1] Handles incoming chat message
  (bind _aslobby_gm (cast `/Game/Blueprints/Lobby/LobbyGM` (`GameplayStatics.GetGameMode`)))
  (for _ (`/Game/Blueprints/Lobby/LobbyGM.AllConnectedPlayers` _aslobby_gm)
    (`/Game/UI/Lobby/ChatWidow.UpdateChatMessage` (`/Game/UI/Lobby/LobbyWB.ChatWidow` (`self.LobbyMenuWB`)) (`.PlayerName_4_399792AF446571371C9F788A93CF97FA` (break `/Game/Blueprints/AllLevels/PlayerInfo` (`self.PlayerInfo`))) MessageToSend)))

(fn `UserConstructionScript`
  (bind _returnvalue (`GameplayStatics.DoesSaveGameExist` "PlayerSaveGame"))
  (if _returnvalue
    (bind _returnvalue_2 (`GameplayStatics.LoadGameFromSlot` "PlayerSaveGame"))
    (bind _output_get (set `self.PlayerSave` _returnvalue_2))
    (bind _asplayer_save_game (cast `/Game/Blueprints/AllLevels/PlayerSaveGame` _output_get))
    (set `self.PlayerInfo` (`/Game/Blueprints/AllLevels/PlayerSaveGame.PlayerInfo` _asplayer_save_game))
    (else
      (`KismetSystemLibrary.PrintString` "Corrupted Save game, please reload the game"))))