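; Lobby game mode that tracks joining players, gives each a character and sends the session to Level01 on launch.
; PostLogin possesses each player with a default Ch_Raven at a random PlayerStart; SwapCharacter replaces that pawn with a chosen class the same way.
; Both then call UpdateEveryone, which rebuilds the PlayerInfo list and pushes it to every LobbyPC.
; LaunchTheGame runs a server-only ServerTravel console command.
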(event `SwapCharacter`
  (params (NewPlayerClass :type "Character Class Reference") (PlayerController :type "Controller Object Reference"))
  (bind _returnvalue (`Controller.K2_GetPawn` PlayerController))
  ;[1 1 1] swap the player
  (`/Engine/EditorBlueprintResources/StandardMacros.IsValid` _returnvalue
    (:`Is Valid`
      (`self.K2_DestroyActor` _returnvalue))
    (:`Is Not Valid`
      _))
  (bind _randomspawnpoint (`self.GetRandomSpawnPoint`))
  (bind _returnvalue_2 (`|SpawnActorFromClass` NewPlayerClass _randomspawnpoint "Undefined" "OverrideRootScale"))
  (`Controller.Possess` PlayerController _returnvalue_2)
  (`self.UpdateEveryone`))

(event `self.K2_PostLogin`
  (params (NewPlayer :type "PlayerController Object Reference"))
  (bind _returnvalue (`Controller.K2_GetPawn` NewPlayer))
  ;[1 1 1] Spawn a base character on entering the lobby
  (`KismetArrayLibrary.Array_Add` (`self.AllConnectedPlayers`) NewPlayer)
  (`KismetArrayLibrary.Array_Add` (`self.ConnectedPlayersInfo`) (`/Game/Blueprints/Lobby/LobbyPC.PlayerInfo` (cast `/Game/Blueprints/Lobby/LobbyPC` NewPlayer :!pure true)))
  (bind _outactors (`GameplayStatics.GetAllActorsOfClass` "/Script/Engine.PlayerStart"))
  (set `self.SpawnPoints` _outactors)
  (`/Engine/EditorBlueprintResources/StandardMacros.IsValid` _returnvalue
    (:`Is Valid`
      (`self.K2_DestroyActor` _returnvalue))
    (:`Is Not Valid`
      _))
  (bind _randomspawnpoint (`self.GetRandomSpawnPoint`))
  (bind _returnvalue_2 (`|SpawnActorFromClass` "/Game/Blueprints/Characters/Ch_Raven.Ch_Raven_C" _randomspawnpoint "Undefined" "OverrideRootScale"))
  (`Controller.Possess` NewPlayer _returnvalue_2)
  (`self.UpdateEveryone`))

(event `LaunchTheGame`
  ;[1 1 1] Launch Level 1
  (if (`KismetSystemLibrary.IsServer`)
    (`KismetSystemLibrary.ExecuteConsoleCommand` "ServerTravel Level01" (`GameplayStatics.GetPlayerController` 0))
    (`KismetSystemLibrary.PrintString` "U*rghh")))

(event `UpdateEveryone`
  (`KismetArrayLibrary.Array_Clear` (`self.ConnectedPlayersInfo`))
  (for _array_element (`self.AllConnectedPlayers`)
    (bind _aslobby_pc (cast `/Game/Blueprints/Lobby/LobbyPC` _array_element))
    (`KismetArrayLibrary.Array_Add` (`self.ConnectedPlayersInfo`) (`/Game/Blueprints/Lobby/LobbyPC.PlayerInfo` _aslobby_pc)))
  (for _array_element_2 (`self.AllConnectedPlayers`)
    (bind _aslobby_pc_2 (cast `/Game/Blueprints/Lobby/LobbyPC` _array_element_2))
    (`/Game/Blueprints/Lobby/LobbyPC.AddPlayerInfo` _aslobby_pc_2 (`self.ConnectedPlayersInfo`))))

(fn `GetRandomSpawnPoint`
  (returns (RandomSpawnPoint :type "Transform Structure"))
  (bind _spawnpoints (`self.SpawnPoints`))
  (return (`self.GetTransform` (`KismetArrayLibrary.Array_Get` _spawnpoints (`KismetMathLibrary.RandomIntegerInRange` 0 (- (`KismetArrayLibrary.Array_Length` _spawnpoints) 1))))))

(fn `UserConstructionScript`)