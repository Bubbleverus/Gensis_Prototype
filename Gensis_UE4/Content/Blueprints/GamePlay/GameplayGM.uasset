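; GameplayGM, apparently the gameplay game mode, spawns the player's last used character and saves their inventory.
; Its construction script loads the PlayerSaveGame slot, if one exists, to set CurrentCharacter.
; BeginPlay destroys the default pawn, then spawns and possesses CurrentCharacter at the first PlayerStart found.
; SaveInventory writes the passed inventory into the save's PlayerInfo struct and saves the slot.
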(event `self.ReceiveBeginPlay`
  ;[1 1 1] Spawn the correct character on begin play
  (`self.K2_DestroyActor` (`GameplayStatics.GetPlayerCharacter` 0))
  (bind _outactors (`GameplayStatics.GetAllActorsOfClass` "/Script/Engine.PlayerStart"))
  (bind _returnvalue (`|SpawnActorFromClass` (`self.CurrentCharacter`) (`self.GetTransform` (`KismetArrayLibrary.Array_Get` _outactors)) "Undefined" "OverrideRootScale"))
  (`Controller.Possess` (`GameplayStatics.GetPlayerController` 0) _returnvalue))

(event `SaveInventory`
  (params (Inventory :type "Array of /Game/Inventory_BP/Item_Structure Structure"))
  ;[1 1 1] Save the player inventory
  (setmembers `/Game/Blueprints/AllLevels/PlayerInfo` :`StructRef` (`/Game/Blueprints/AllLevels/PlayerSaveGame.PlayerInfo` (cast `/Game/Blueprints/AllLevels/PlayerSaveGame` (`self.playerSaveGame`) :!pure true)) :`SavedInventory` Inventory)
  (`GameplayStatics.SaveGameToSlot` (`self.playerSaveGame`) "PlayerSaveGame"))

(fn `UserConstructionScript`
  (bind _returnvalue (`GameplayStatics.DoesSaveGameExist` "PlayerSaveGame"))
  (if _returnvalue
    (`KismetSystemLibrary.PrintString` "yes saved game")
    (bind _returnvalue_2 (`GameplayStatics.LoadGameFromSlot` "PlayerSaveGame"))
    (bind _output_get (set `self.playerSaveGame` _returnvalue_2))
    (bind _asplayer_save_game (cast `/Game/Blueprints/AllLevels/PlayerSaveGame` _output_get))
    (set `self.CurrentCharacter` (`.LastUsedCharacter_6_8210F8E347007A5B69137FA8083158B7` (break `/Game/Blueprints/AllLevels/PlayerInfo` (`/Game/Blueprints/AllLevels/PlayerSaveGame.PlayerInfo` _asplayer_save_game))))
    (else
      (`KismetSystemLibrary.PrintString` "no saved game"))))