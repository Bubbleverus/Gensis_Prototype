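; Main menu game mode, judging by its name, that handles LAN multiplayer sessions through host, search, join and destroy events.
; Hosting creates a session with zero public connections and opens Lobby as a listen server.
; Search requests one result and stores it from the async node's immediate Then output, not On Success.
; Join uses the first stored result unchecked and sets JoinedSession, with every event printing failures on screen.
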(event `HostGame`
  ;[1 1 1] Host Game
  (`CreateSessionCallbackProxy.CreateSession` (`GameplayStatics.GetPlayerController` 0) 0 true
    (:`OnSuccess`
      (`KismetSystemLibrary.ExecuteConsoleCommand` "open Lobby?listen")
      (`KismetSystemLibrary.PrintString` "Created Session"))
    (:`OnFailure`
      (`KismetSystemLibrary.PrintString` "Failed to create session"))))

(event `SearchGame`
  ;[1 1 1] Search for a session to play
  (bind _results (`FindSessionsCallbackProxy.FindSessions` (`GameplayStatics.GetPlayerController` 0) 1 true)
    (:`then`
      (set `self.SessionFound` _results))
    (:`OnFailure`
      (`KismetSystemLibrary.PrintString` "Unable to find a session"))))

(event `JoinGame`
  ;[1 1 1] Joining a session
  (`JoinSessionCallbackProxy.JoinSession` (`GameplayStatics.GetPlayerController` 0) (`KismetArrayLibrary.Array_Get` (`self.SessionFound`))
    (:`OnSuccess`
      (`KismetSystemLibrary.PrintString` "Joined a session")
      (set `self.JoinedSession` true))
    (:`OnFailure`
      (`KismetSystemLibrary.PrintString` "Failed to join a session")
      (set `self.JoinedSession` false))))

(event `DestroySession`
  ;[1 1 1] Destroy current session
  (`DestroySessionCallbackProxy.DestroySession` (`GameplayStatics.GetPlayerController` 0)
    (:`OnSuccess`
      (`KismetSystemLibrary.PrintString` "Destroyed session"))
    (:`OnFailure`
      (`KismetSystemLibrary.PrintString` "Unable to destroy session"))))