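; Sol character Blueprint that gives the player a timed Eagle Vision screen effect.
; BeginPlay adds an unbound post process component and registers a dynamic instance of the Eagle Vision material as a blendable at zero weight.
; Pressing ActivateAbility restarts the WeightGraph timeline, which drives the blendable's weight and resets it to zero when finished.
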(event `self.ReceiveBeginPlay`
  ;[1 1 1] On begin play - creates a post process volume ready for when eagle vision is needed
  (bind _returnvalue (`AddComponent|NODE_AddPostProcessComponent-2`))
  (bind _output_get (set `self.PostProcess` _returnvalue))
  (set `PostProcessComponent.bUnbound` true _output_get)
  (bind _returnvalue_2 (`KismetMaterialLibrary.CreateDynamicMaterialInstance` "/Game/Mannequin/Character/Materials/EagleVision/EagleVisionMAt_Inst.EagleVisionMAt_Inst"))
  (bind _output_get_2 (set `self.ev_mat_ref` _returnvalue_2))
  (`PostProcessComponent.AddOrUpdateBlendable` (`self.PostProcess`) _output_get_2 0.0))

(event `InputAction|ActivateAbility`
  (params (Key :type "Key Structure" :default "AnyKey"))
  ;[1 1 1] Updates the Weight of the eagle vision - (turning it on and off)
  (:`Pressed`
    (bind (_direction _abilityweight) (`Timeline|WeightGraph` :!via `PlayFromStart`)
      (:`Update`
        (`PostProcessComponent.AddOrUpdateBlendable` (`self.PostProcess`) (`self.ev_mat_ref`) _abilityweight))
      (:`Finished`
        (`PostProcessComponent.AddOrUpdateBlendable` (`self.PostProcess`) (`self.ev_mat_ref`) 0.0)))))

(fn `UserConstructionScript`
  (`parent.UserConstructionScript`))