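; Base character Blueprint that handles sprinting, an inventory toggle and proximity interaction.
; Sprint input swaps walk speed, and Inventory input creates or removes the Inventory_UI widget, restoring game-only input on close.
; When the capsule overlaps a SampleClass actor, a sphere query sends InteractMessage to nearby WorldDynamic actors implementing Interaction_Bp.
; Tick draws a debug camera-forward visibility trace whose result drives nothing.
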(event `InputAction|Sprint`
  (params (Key :type "Key Structure" :default "AnyKey"))
  (bind _charactermovement (`self.CharacterMovement`))
  (:`Pressed`
    (set `CharacterMovementComponent.MaxWalkSpeed` (`self.sprint_speed`) _charactermovement))
  (:`Released`
    (set `CharacterMovementComponent.MaxWalkSpeed` (`self.walk_speed`) _charactermovement)))

(event `self.ReceiveTick`
  (params (DeltaSeconds :type "Float (single-precision)"))
  (bind _returnvalue (`SceneComponent.K2_GetComponentLocation` (`self.FollowCamera`)))
  (bind _outhit (`KismetSystemLibrary.LineTraceSingle` :`Start` _returnvalue :`End` (+ _returnvalue (* (`SceneComponent.GetForwardVector` (`self.FollowCamera`)) 5000.0)) :`TraceChannel` "TraceTypeQuery1" :`DrawDebugType` "ForOneFrame")))

(event `InputAction|Inventory` :paused true
  (params (Key :type "Key Structure" :default "AnyKey"))
  ;[1 1 1] Use I for open close inventory
  (:`Pressed`
    (if (`self.InventoryOpen`)
      (`Widget.RemoveFromParent` (stale _returnvalue))
      (`WidgetBlueprintLibrary.SetInputMode_GameOnly` (`GameplayStatics.GetPlayerController` 0))
      (set `self.InventoryOpen` false)
      (set `PlayerController.bShowMouseCursor` false (`GameplayStatics.GetPlayerController` 0))
      (else
        (bind _returnvalue (`|CreateWidget` "/Game/Inventory_BP/Inventory_UI.Inventory_UI_C" null null 0 false "NewEnumerator0"))
        (set `self.InventoryOpen` true)
        (`UserWidget.AddToViewport` _returnvalue 0)))))

(event `self.CapsuleComponent.OnComponentBeginOverlap`
  (params (OverlappedComponent :type "PrimitiveComponent Object Reference") (OtherActor :type "Actor Object Reference") (OtherComp :type "PrimitiveComponent Object Reference") (OtherBodyIndex :type Integer) (bFromSweep :type Boolean) (SweepResult :type "HitResult Structure (by ref)"))
  (cast `/Game/Inventory_BP/SampleClass` OtherActor)
  (bind _outactors (`KismetSystemLibrary.SphereOverlapActors_NEW` (`self.K2_GetActorLocation`) 200.0 (`|MakeArray` "ObjectTypeQuery2" :!type "EObjectTypeQuery Enum")))
  (for _array_element _outactors
    (if (`KismetSystemLibrary.DoesImplementInterface` _array_element "/Game/Inventory_BP/Interaction_Bp.Interaction_Bp_C")
      (message `/Game/Inventory_BP/Interaction_Bp.Interact` _array_element self))))

(fn `UserConstructionScript`)