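; Remi character Blueprint whose custom ability toggles invisibility.
; BeginPlay caches the mesh's materials in PrevMats.
; CustomAbility reads AbilityActive to set IsVisible and loop over the cached slots, creating dynamic instances from InvisibleMaterial when active or from the saved materials when inactive.
; The BeginPlay note about an eagle vision post process volume does not match its logic, which only caches materials.
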(event `self.ReceiveBeginPlay`
  ;[1 1 1] On begin play - creates a post process volume ready for when eagle vision is needed
  (set `self.prev_mats` (`MeshComponent.GetMaterials` (`self.Mesh`))))

(event `self.CustomAbility`
  ;[1 1 1] Invisibility Function
  (if (`self.abilityActive?`)
    (set `self.IsVisible?` false)
    (for (_ _array_index) (`self.prev_mats`)
      (`PrimitiveComponent.CreateDynamicMaterialInstance` (`self.Mesh`) _array_index (`self.InvisibleMaterial`)))
    (else
      (set `self.IsVisible?` true)
      (for (_array_element _array_index_2) (`self.prev_mats`)
        (`PrimitiveComponent.CreateDynamicMaterialInstance` (`self.Mesh`) _array_index_2 _array_element)))))

(fn `NewFunction_0_0`)

(fn `UserConstructionScript`
  (`parent.UserConstructionScript`))