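; Base weapon Blueprint providing automatic hitscan fire, automatic reload and a world-space crosshair.
; StartFiring and StopFiring toggle a Tick-driven gate, where delays pace shots and trigger a timed reload once the magazine empties.
; Each shot plays a sound, prints debug text and applies damage along a debug-drawn trace from GunDirection.
; Every tick another trace positions the crosshair just short of the aimed surface, and PickupWeapon simply destroys the actor.
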(event `Firing`
  (bind _gundirection (`self.GunDirection`))
  (bind _returnvalue (`SceneComponent.K2_GetComponentLocation` _gundirection))
  ;[1 1 1] Firing
  (`GameplayStatics.PlaySoundAtLocation` (`self.Sound`) (`self.K2_GetActorLocation` (`GameplayStatics.GetPlayerCharacter` 0)) (struct))
  (`KismetSystemLibrary.PrintString` "Bang Bang your gonna die")
  (bind _outhit (`KismetSystemLibrary.LineTraceSingle` :`Start` _returnvalue :`End` (+ _returnvalue (* (`SceneComponent.GetForwardVector` _gundirection) (`self.Range`))) :`TraceChannel` "TraceTypeQuery1" :`DrawDebugType` "ForDuration"))
  (`GameplayStatics.ApplyDamage` (`.HitActor` (`GameplayStatics.BreakHitResult` _outhit)) (`self.Damage`) (`self.GetInstigatorController`) self))

(event `self.ReceiveTick`
  (params (DeltaSeconds :type "Float (single-precision)"))
  ;[1 1 1] Creating the Crosshair
  (`self.DrawCrosshair`)
  (`/Engine/EditorBlueprintResources/StandardMacros.Gate` true :!label _label
    (:`Exit`
      (if (> (`self.MagSize`) 0)
        (`KismetSystemLibrary.Delay` (`self.FireDelay`))
        (set `self.MagSize` (- (`self.MagSize`) 1))
        (`self.Firing`)
        (else
          (`KismetSystemLibrary.Delay` 3.0)
          (`GameplayStatics.PlaySoundAtLocation` (`self.ReloadSound`) (`self.K2_GetActorLocation` (`GameplayStatics.GetPlayerCharacter` 0)))
          (set `self.MagSize` (`self.MaxMagSize`)))))))

(event `StartFiring`
  ;[1 1 1] Creating the Crosshair
  (goto _label :!via `Open`))

(event `StopFiring`
  ;[1 1 1] Creating the Crosshair
  (goto _label :!via `Close`))

(event `PickupWeapon`
  (`self.K2_DestroyActor`))

(fn `DrawCrosshair`
  (bind _gundirection (`self.GunDirection`))
  (bind _crosshair (`self.CrossHair`))
  (bind _returnvalue (`SceneComponent.K2_GetComponentLocation` _gundirection))
  (bind (_outhit _returnvalue_2) (`KismetSystemLibrary.LineTraceSingle` _returnvalue (+ _returnvalue (* (`SceneComponent.GetForwardVector` _gundirection) 100000)) "TraceTypeQuery1"))
  (if _returnvalue_2
    (`SceneComponent.K2_SetWorldLocation` _crosshair (- (`.Location` (`GameplayStatics.BreakHitResult` _outhit)) (* (`SceneComponent.GetForwardVector` (`self.GunDirection`)) 10.0)) false false)
    (else
      (`SceneComponent.K2_SetWorldLocation` _crosshair (* (`SceneComponent.GetForwardVector` (`self.GunDirection`)) 10) false false))))

(fn `NewFunction_0`
  (set `self.WeaponStats` (struct)))

(fn `UserConstructionScript`
  (bind _output_get (set `self.WeaponStats` (make `/Game/Inventory_BP/WeaponStructure` (`self.Damage`) (`KismetMathLibrary.Conv_IntToDouble` (`self.Range`)) (`KismetMathLibrary.Conv_IntToDouble` (`self.MagSize`)) (`self.FireDelay`))))
  (set `self.WeaponStats` _output_get))